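; Ghost trail actor that shows a snapshot of the player character's pose on a poseable mesh.
; On BeginPlay it caches player 0's character, then for each mesh material creates and stores a dynamic instance, copies the pose and starts the Opacity timeline.
; The timeline's update is meant to drive each instance's Opacity parameter.
; A DestroyActor node is present but unconnected, so the actor never removes itself.
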(event Custom|Ghostrail
  (for _array_element (Rendering|Material|GetMaterials (Variables|Default|GetPoseableMesh))
    (bind _returnvalue (Rendering|Material|CreateDynamicMaterialInstance 0 "None" :!class /Script/Engine.KismetMaterialLibrary))
    (bind _returnvalue_2 (Utilities|Array|Add (Variables|Default|GetDynamicMats) _returnvalue))
    (Rendering|Material|SetMaterial (Variables|Default|GetPoseableMesh) _returnvalue_2 _returnvalue)
    (Class|PoseableMeshComponent|CopyPosefromSkeletalComponent (Variables|Default|GetPoseableMesh) (Variables|/Script/Engine.Character|GetMesh (Variables|Default|GetPlayerCharacter%20Ref)))
    (Components|Timeline|PlayfromStart (Variables|Colors|GetOpacity))))

(event EventBeginPlay
  (bind _ascharacter (Utilities|Casting|CastToCharacter (Game|Player|GetPlayerPawn 0)))
  (Variables|Default|SetPlayerCharacter%20Ref _ascharacter)
  (CallFunction|Ghostrail))

(fn ConstructionScript)