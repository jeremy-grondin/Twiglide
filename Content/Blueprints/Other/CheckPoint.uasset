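; Checkpoint actor that records a respawn point for the player character and restores health on first use.
; On overlap with a PlayerCharacter, the IsUsed flag gates a one-time refill of Life to MaxLife.
; Every such overlap writes the actor's location to the player's CheckPointLocation and calls SetMaterial on the first material slot of the Cylinder.
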(event EventBeginPlay)

(event Collision|EventActorBeginOverlap
  (params (OtherActor :type Actor%20Object%20Reference))
  (bind _asplayer_character (Utilities|Casting|CastToPlayerCharacter OtherActor))
  (if (Variables|Default|GetIsUsed)
    _
    (else
      (Variables|Default|SetIsUsed true)
      (Variables|/Script/Twiglide.GenericCharacter|Setlife _asplayer_character (Variables|/Script/Twiglide.GenericCharacter|GetmaxLife _asplayer_character))))
  (Variables|/Script/Twiglide.PlayerCharacter|SetcheckPointLocation _asplayer_character (Transformation|GetActorLocation self))
  (Rendering|Material|SetMaterial (Variables|Default|GetCylinder) 0 0))

(event EventTick
  (params (DeltaSeconds :type Float%20%28single-precision%29)))

(fn ConstructionScript)