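; Archer enemy Blueprint that can show a target marker and fire arrows.
; Tick shows or hides the TargetVisual component every frame based on the IsTargeted flag.
; DistanceFromPlayerCheck returns the distance to the first player's character, and FireArrow spawns an Arrow at the archer's own transform.
; Neither function is called within this Blueprint's graphs, and nothing here sets IsTargeted.
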(event EventTick
  (params (DeltaSeconds :type Float%20%28single-precision%29))
  (bind _targetvisual (Variables|Default|GetTargetVisual))
  (if (Variables|Default|GetisTargeted)
    (Development|SetHiddeninGame _targetvisual false false)
    (else
      (Development|SetHiddeninGame _targetvisual true false))))

(fn ConstructionScript)

(fn DistancefromPlayerCheck
  (return (Transformation|GetDistanceTo (Game|GetPlayerCharacter 0))))

(fn FireArrow
  (Game|SpawnActorfromClass "/Game/Blueprints/Enemy/Arrow.Arrow_C" (Transformation|GetActorTransform self) "Undefined" 0 0))